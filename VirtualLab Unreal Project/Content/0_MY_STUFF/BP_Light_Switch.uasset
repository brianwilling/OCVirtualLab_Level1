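; Wall light switch Blueprint that toggles a connected ceiling light on and off when its Combine event fires.
; Combine branches on the connected light's IsOn flag, tilts or resets the Switch component, and prints a debug message.
; It then sets the RectLight intensity to zero or the light's ONIntensity, swaps the lamp's on/off material, and updates IsOn on the light itself.
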(event EventCombine
  (params (HitComp :type Primitive%20Component%20Object%20Reference) (PhysicsHandle :type Physics%20Handle%20Component%20Object%20Reference))
  (bind _connected_light (Variables|Default|GetConnected%20Light))
  (if (Variables|/Game/0_MY_STUFF/BP_Ceiling_Lamp.BP_Ceiling_Lamp_C|GetIsOn (Variables|Default|GetConnected%20Light))
    (Transformation|SetRelativeRotation (Variables|Default|GetSwitch) "0.000000, 0,-5.000000" false false)
    (Development|PrintString "Turn OFF Ceiling Light" true true "(R=1.000000,G=0.076844,B=0.000000,A=1.000000)")
    (Rendering|Components|Light|SetIntensity (Variables|/Game/0_MY_STUFF/BP_Ceiling_Lamp.BP_Ceiling_Lamp_C|GetRectLight (Variables|Default|GetConnected%20Light)) 0.0)
    (Rendering|Material|SetMaterial (Variables|/Game/0_MY_STUFF/BP_Ceiling_Lamp.BP_Ceiling_Lamp_C|GetLamp (Variables|Default|GetConnected%20Light)) 2 "/Game/0_MY_STUFF/ceiling_lamp_off.ceiling_lamp_off")
    (Variables|/Game/0_MY_STUFF/BP_Ceiling_Lamp.BP_Ceiling_Lamp_C|SetIsOn (Variables|Default|GetConnected%20Light) false)
    (else
      (Transformation|SetRelativeRotation (Variables|Default|GetSwitch) "0, 0, 0" false false)
      (Development|PrintString "Turn ON ceiling light" true true "(R=0.000000,G=1.000000,B=0.302208,A=1.000000)")
      (Rendering|Components|Light|SetIntensity (Variables|/Game/0_MY_STUFF/BP_Ceiling_Lamp.BP_Ceiling_Lamp_C|GetRectLight _connected_light) (Variables|/Game/0_MY_STUFF/BP_Ceiling_Lamp.BP_Ceiling_Lamp_C|GetON%20Intensity _connected_light))
      (Rendering|Material|SetMaterial (Variables|/Game/0_MY_STUFF/BP_Ceiling_Lamp.BP_Ceiling_Lamp_C|GetLamp (Variables|Default|GetConnected%20Light)) 2 "/Game/0_MY_STUFF/ceiling_lamp_on.ceiling_lamp_on")
      (Variables|/Game/0_MY_STUFF/BP_Ceiling_Lamp.BP_Ceiling_Lamp_C|SetIsOn (Variables|Default|GetConnected%20Light) true))))

(fn ConstructionScript)