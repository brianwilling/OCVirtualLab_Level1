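; BP_Rolling_Cupboard is a cupboard whose drawers slide open and closed when hit through its Combine event.
; Each direct child of Frame is a drawer, matched by index to the IsOpen array.
; Combine toggles the hit drawer by snapping its relative X between zero and SlideDistance, printing the new state.
; The construction script applies the same offset to drawers flagged open, previewing their starting state.
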(event EventCombine
  (params (HitComp :type Primitive%20Component%20Object%20Reference) (PhysicsHandle :type Physics%20Handle%20Component%20Object%20Reference))
  (bind _relativelocation (Variables|/Script/Engine.SceneComponent|GetRelativeLocation HitComp))
  (bind _frame (Variables|Default|GetFrame))
  (bind _isopen (Variables|Default|GetIsOpen))
  (bind _children (Components|GetChildrenComponents _frame false))
  (bind _returnvalue (Utilities|Array|FindItem _children HitComp))
  (if (Utilities|Array|ContainsItem _children HitComp)
    (if (Utilities|Array|Get(acopy) _isopen _returnvalue)
      (Transformation|SetRelativeLocation HitComp (Math|Vector|MakeVector 0.0 (.y _relativelocation) (.z _relativelocation)) false false)
      (Utilities|Array|SetArrayElem _isopen _returnvalue false)
      (Development|PrintString "is closed")
      (else
        (Transformation|SetRelativeLocation HitComp (Math|Vector|MakeVector (Variables|Default|GetSlideDistance) (.y _relativelocation) (.z _relativelocation)) false false)
        (Utilities|Array|SetArrayElem _isopen _returnvalue true)
        (Development|PrintString "is open")))))

(fn ConstructionScript
  ;[1 1 1] Create the arrays for the properties of the drawers (drawer refs, is open, slide distance)
  (for (_array_element _array_index) (Components|GetChildrenComponents (Variables|Default|GetFrame) false)
    (if (Utilities|Array|Get(acopy) (Variables|Default|GetIsOpen) _array_index)
      (Transformation|SetRelativeLocation _array_element (Math|Vector|MakeVector (Variables|Default|GetSlideDistance) (.y (Variables|/Script/Engine.SceneComponent|GetRelativeLocation _array_element)) (.z (Variables|/Script/Engine.SceneComponent|GetRelativeLocation _array_element))) false false))))