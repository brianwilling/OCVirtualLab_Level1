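; Interaction component that detects the interaction area the player looks at and triggers interaction with it.
; Each tick it line-traces forward from the camera on the Visibility channel, toggling focus on BP_Interaktionsarea hits as the target changes.
; TryToInteract passes a focused area to InteractOnServer only when its InteractDuration is not positive; timed interactions are not handled here.
; InteractOnServer sends the interface interact message to the area's parent actor.
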(event Custom|TryToInteract
  (params (In :type Boolean))
  (if In
    (if (Variables|Default|GetisTracingInteractionArea)
      (bind _output_get (Variables|Default|SetInteract%20Duration (Variables|/Game/0_MY_STUFF/Interaktion/Interaktionsarea/BP_Interaktionsarea.BP_Interaktionsarea_C|GetInteractDuration (Variables|Default|GetFocusedInteractionArea))))
      (if (not (> _output_get 0.0))
        (CallFunction|InteractonServer (Variables|Default|GetFocusedInteractionArea))))))

(event Custom|InteractOnServer
  (params (InteractionArea :type BP%20Interaktionsarea%20Object%20Reference))
  (Class|BIInteraktion|InterfaceInteract(Message) (Actor|GetParentActor InteractionArea)))

(event EventTick
  (params (DeltaSeconds :type Float%20%28single-precision%29))
  (CallFunction|Trace))

(fn Trace
  (bind _returnvalue (Game|GetPlayerCameraManager 0))
  (bind _returnvalue_2 (Transformation|GetActorLocation _returnvalue))
  (bind (_outhit _returnvalue_3) (Collision|LineTraceByChannel _returnvalue_2 (+ _returnvalue_2 (* (Math|Vector|GetForwardVector (Transformation|GetActorRotation _returnvalue)) (Variables|Default|GetLaenge))) "TraceTypeQuery1" false 0 "None"))
  (if _returnvalue_3
    (if (!= (Variables|Default|GetfocusedActor) (.HitActor (Collision|BreakHitResult _outhit)))
      (Variables|Default|SetfocusedActor (.HitActor (Collision|BreakHitResult _outhit)))
      (CallFunction|TraceInteraktionsarea (== (Utilities|GetClass (.HitActor (Collision|BreakHitResult _outhit))) "/Game/0_MY_STUFF/Interaktion/Interaktionsarea/BP_Interaktionsarea.BP_Interaktionsarea_C")))
    (else
      (CallFunction|TraceInteraktionsarea false))))

(fn TraceInteraktionsarea
  (params (Trace :type Boolean))
  (if Trace
    (if (Variables|Default|GetisTracingInteractionArea)
      (Default|ToggleFocus (Variables|Default|GetFocusedInteractionArea) false))
    (bind _asbp_interaktionsarea (Utilities|Casting|CastToBP_Interaktionsarea (Variables|Default|GetfocusedActor)))
    (bind _output_get (Variables|Default|SetFocusedInteractionArea _asbp_interaktionsarea))
    (Default|ToggleFocus _output_get true)
    (Variables|Default|SetisTracingInteractionArea true)
    (elif (Variables|Default|GetisTracingInteractionArea)
      (Variables|Default|SetisTracingInteractionArea false)
      (Default|ToggleFocus (Variables|Default|GetFocusedInteractionArea) false)
      (Variables|Default|SetfocusedActor 0)
      (Variables|Default|SetFocusedInteractionArea 0))))