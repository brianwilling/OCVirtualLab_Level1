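; BP_UV_Lamp is a UV lamp that holds papers and reveals their BP_DC_Dot decals while lit.
; Combine moves a paper from held tweezers (BP_Pinzette) onto numbered sockets, returns the last to empty tweezers, or falls through to Ping for occupied slots.
; Ping toggles the RectLight and syncs decal visibility on each attached paper.
; An older single-paper Combine remains as unconnected nodes.
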(event Custom|Set%20Decal%20Visibility%20BP_UV_Lamp
  (params (Visible :type Boolean) (Paper :type Actor%20Object%20Reference))
  (bind _outactors (Actor|GetAttachedActors Paper true false))
  (if (> (Utilities|Array|Length _outactors) 0)
    (for _array_element _outactors
      (bind _asbp_dc_dot (Utilities|Casting|CastToBP_DC_Dot _array_element))
      (Rendering|SetVisibility (Variables|/Script/Engine.DecalActor|GetDecal _asbp_dc_dot) Visible false))))

(event EventPing
  (if (Variables|Default|GetIsOn)
    (Rendering|Components|Light|SetIntensity (Variables|Default|GetRectLight) 0.0)
    (bind _output_get (Variables|Default|SetIsOn false))
    (for (_array_element _array_index) (Variables|Default|GetLampHasPaper_Array)
      (if _array_element
        (CallFunction|SetDecalVisibilityBPUVLamp _output_get (Utilities|Array|Get(acopy) (Variables|Default|GetAttachted_Paper_Array) _array_index))))
    (else
      (Rendering|Components|Light|SetIntensity (Variables|Default|GetRectLight) (Variables|Default|GetON%20Intensity))
      (bind _output_get_2 (Variables|Default|SetIsOn true))
      (for (_array_element_2 _array_index_2) (Variables|Default|GetLampHasPaper_Array)
        (if _array_element_2
          (CallFunction|SetDecalVisibilityBPUVLamp _output_get_2 (Utilities|Array|Get(acopy) (Variables|Default|GetAttachted_Paper_Array) _array_index_2)))))))

(event EventCombine
  (params (HitComp :type Primitive%20Component%20Object%20Reference) (PhysicsHandle :type Physics%20Handle%20Component%20Object%20Reference))
  (bind _attachted_paper_array (Variables|Default|GetAttachted_Paper_Array))
  ;[1 1 1] Find out situation
  (Variables|Default|SetPinzetteHasPaper (CallFunction|GetPinzetteHasPaper))
  (Variables|Default|SetIsHoldingPinzette (CallFunction|GetIsHoldingPinzette))
  ;[1 1 1] Attach Paper if true
  (if (and (Variables|Default|GetIsHoldingPinzette) (Variables|Default|GetPinzetteHasPaper))
    (Utilities|Array|Add (Variables|Default|GetAttachted_Paper_Array) (Utilities|Array|Get(acopy) (Actor|GetAttachedActors (CallFunction|GetHeldActor) true false)))
    (Variables|Default|SetAnzahl_Paper (+ 1 (Variables|Default|GetAnzahl_Paper)))
    (Transformation|AttachActorToActor (Utilities|Array|Get(acopy) (Variables|Default|GetAttachted_Paper_Array) (- (Variables|Default|GetAnzahl_Paper) 1)) self (Utilities|String|StringToName (Utilities|String|ToString(Integer) (Variables|Default|GetAnzahl_Paper))) "SnapToTarget" "SnapToTarget" "SnapToTarget" true)
    (Utilities|Array|SetArrayElem (Variables|Default|GetLampHasPaper_Array) (- (Variables|Default|GetAnzahl_Paper) 1) true true)
    (for _array_element (Variables|Default|GetAttachted_Paper_Array)
      (if (Variables|Default|GetIsOn)
        (CallFunction|SetDecalVisibilityBPUVLamp true _array_element)
        (else
          (CallFunction|SetDecalVisibilityBPUVLamp false _array_element))))
    (else
      (bind _array_element_2 (Utilities|Array|ForEachLoopwithBreak (Variables|Default|GetLampHasPaper_Array))
        (:LoopBody
          (if _array_element_2
            ;[1 1 1] Detach Paper if True
            (if (Math|Boolean|ANDBoolean _array_element_2 (not (Variables|Default|GetPinzetteHasPaper)) (Variables|Default|GetIsHoldingPinzette))
              (Transformation|AttachActorToActor (Utilities|Array|Get(acopy) (Actor|GetAttachedActors true false) (- (Variables|Default|GetAnzahl_Paper) 1)) (CallFunction|GetHeldActor) "Paper" "SnapToTarget" "SnapToTarget" "SnapToTarget" true)
              (Utilities|Array|SetArrayElem (Variables|Default|GetLampHasPaper_Array) (- (Variables|Default|GetAnzahl_Paper) 1) false)
              (CallFunction|SetDecalVisibilityBPUVLamp false (Utilities|Array|Get(acopy) _attachted_paper_array (- (Variables|Default|GetAnzahl_Paper) 1)))
              (Utilities|Array|SetArrayElem _attachted_paper_array (- (Variables|Default|GetAnzahl_Paper) 1) 0) ; Clear Element
              (Variables|Default|SetAnzahl_Paper (- (Variables|Default|GetAnzahl_Paper) 1))
              (else
                (CallFunction|Ping)))))))))

(fn ConstructionScript
  (if (Variables|Default|GetIsOn)
    (Rendering|Components|Light|SetIntensity (Variables|Default|GetRectLight) (Variables|Default|GetON%20Intensity))
    (Development|PrintString "is on")))

(fn GetPinzetteHasPaper
  (if (CallFunction|PlayerIsHolding)
    (if (== (Utilities|GetClass (CallFunction|GetHeldActor)) "/Game/0_MY_STUFF/BP_Pinzette.BP_Pinzette_C")
      (if (== (Utilities|Array|Length (Actor|GetAttachedActors (CallFunction|GetHeldActor) true false)) 1)
        (if (== (Utilities|GetClass (Utilities|Array|Get(acopy) (Actor|GetAttachedActors (CallFunction|GetHeldActor) true false))) "/Game/0_MY_STUFF/BP_Paper.BP_Paper_C")
          (return true)
          (else
            (return false)))
        (else
          (return false)))
      (else
        (return false)))
    (else
      (return false))))

(fn GetIsHoldingPinzette
  (if (CallFunction|PlayerIsHolding)
    (if (== (Utilities|GetClass (CallFunction|GetHeldActor)) "/Game/0_MY_STUFF/BP_Pinzette.BP_Pinzette_C")
      (return true)
      (else
        (return false)))
    (else
      (return false))))