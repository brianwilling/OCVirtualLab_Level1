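; UV lamp that takes a paper from held tweezers (BP_Pinzette) and reveals the dot decals on it while switched on.
; Combine moves the paper between the tweezers' and lamp's "Paper" sockets, otherwise falls through to Ping.
; Ping toggles the RectLight intensity and, with paper loaded, sets decal visibility on its attached BP_DC_Dot actors.
; Helper functions identify held tweezers and paper through class checks and attached-actor queries.
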(event Custom|Set%20Decal%20Visibility%20BP_UV_Lamp
  (params (Visible :type Boolean) (Paper :type Actor%20Object%20Reference))
  (bind _outactors (Actor|GetAttachedActors Paper true false))
  (if (> (Utilities|Array|Length _outactors) 0)
    (for _array_element _outactors
      (bind _asbp_dc_dot (Utilities|Casting|CastToBP_DC_Dot _array_element))
      (Rendering|SetVisibility (Variables|/Script/Engine.DecalActor|GetDecal _asbp_dc_dot) Visible false))))

(event EventPing
  (if (Variables|Default|GetIsOn)
    (Rendering|Components|Light|SetIntensity (Variables|Default|GetRectLight) 0.0)
    (bind _output_get (Variables|Default|SetIsOn false))
    (if (Variables|Default|GetLampHasPaper)
      (CallFunction|SetDecalVisibilityBPUVLamp _output_get (Variables|Default|GetAttached%20Paper)))
    (else
      (Rendering|Components|Light|SetIntensity (Variables|Default|GetRectLight) (Variables|Default|GetON%20Intensity))
      (bind _output_get_2 (Variables|Default|SetIsOn true))
      (if (Variables|Default|GetLampHasPaper)
        (CallFunction|SetDecalVisibilityBPUVLamp _output_get_2 (Variables|Default|GetAttached%20Paper))))))

(event EventCombine
  (params (HitComp :type Primitive%20Component%20Object%20Reference) (PhysicsHandle :type Physics%20Handle%20Component%20Object%20Reference))
  ;[1 1 1] Find out situation
  (Variables|Default|SetPinzetteHasPaper (CallFunction|GetPinzetteHasPaper))
  (Variables|Default|SetIsHoldingPinzette (CallFunction|GetIsHoldingPinzette))
  ;[1 1 1] Attach Paper if true
  (if (Math|Boolean|ANDBoolean (not (Variables|Default|GetLampHasPaper)) (Variables|Default|GetPinzetteHasPaper) (Variables|Default|GetIsHoldingPinzette))
    (bind _output_get (Variables|Default|SetAttached%20Paper (Utilities|Array|Get(acopy) (Actor|GetAttachedActors (CallFunction|GetHeldActor) true false))))
    (Transformation|AttachActorToActor _output_get self "Paper" "SnapToTarget" "SnapToTarget" "SnapToTarget" true)
    (Variables|Default|SetLampHasPaper true)
    (if (Variables|Default|GetIsOn)
      (CallFunction|SetDecalVisibilityBPUVLamp true (Variables|Default|GetAttached%20Paper))
      (else
        (CallFunction|SetDecalVisibilityBPUVLamp false (Variables|Default|GetAttached%20Paper))))
    (else
      ;[1 1 1] Detach Paper if True
      (if (Math|Boolean|ANDBoolean (Variables|Default|GetLampHasPaper) (not (Variables|Default|GetPinzetteHasPaper)) (Variables|Default|GetIsHoldingPinzette))
        (Transformation|AttachActorToActor (Utilities|Array|Get(acopy) (Actor|GetAttachedActors true false)) (CallFunction|GetHeldActor) "Paper" "SnapToTarget" "SnapToTarget" "SnapToTarget" true)
        (Variables|Default|SetLampHasPaper false)
        (CallFunction|SetDecalVisibilityBPUVLamp false (Variables|Default|GetAttached%20Paper))
        ;[1 1 1] Clear Actor reference
        (Variables|Default|SetAttached%20Paper 0)
        (else
          (CallFunction|Ping))))))

(fn ConstructionScript
  (if (Variables|Default|GetIsOn)
    (Rendering|Components|Light|SetIntensity (Variables|Default|GetRectLight) (Variables|Default|GetON%20Intensity))
    (Development|PrintString "is on")))

(fn GetPinzetteHasPaper
  (if (CallFunction|PlayerIsHolding)
    (if (== (Utilities|GetClass (CallFunction|GetHeldActor)) "/Game/0_MY_STUFF/BP_Pinzette.BP_Pinzette_C")
      (if (== (Utilities|Array|Length (Actor|GetAttachedActors (CallFunction|GetHeldActor) true false)) 1)
        (if (== (Utilities|GetClass (Utilities|Array|Get(acopy) (Actor|GetAttachedActors (CallFunction|GetHeldActor) true false))) "/Game/0_MY_STUFF/BP_Paper.BP_Paper_C")
          (return true)
          (else
            (return false)))
        (else
          (return false)))
      (else
        (return false)))
    (else
      (return false))))

(fn GetIsHoldingPinzette
  (if (CallFunction|PlayerIsHolding)
    (if (== (Utilities|GetClass (CallFunction|GetHeldActor)) "/Game/0_MY_STUFF/BP_Pinzette.BP_Pinzette_C")
      (return true)
      (else
        (return false)))
    (else
      (return false))))