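; Ceiling lamp Blueprint whose lit or unlit state is set by the IsOn flag.
; The construction script sets the rect light to ONIntensity or zero and swaps material slot 2 of the lamp mesh between on and off materials to match.
; Both branches print the same "is on" debug string, including the off branch.
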(fn ConstructionScript
  (if (Variables|Default|GetIsOn)
    (Rendering|Components|Light|SetIntensity (Variables|Default|GetRectLight) (Variables|Default|GetON%20Intensity))
    (Rendering|Material|SetMaterial (Variables|Default|GetLamp) 2 "/Game/0_MY_STUFF/ceiling_lamp_on.ceiling_lamp_on")
    (Development|PrintString "is on")
    (else
      (Rendering|Components|Light|SetIntensity (Variables|Default|GetRectLight) 0.0)
      (Rendering|Material|SetMaterial (Variables|Default|GetLamp) 2 "/Game/0_MY_STUFF/ceiling_lamp_off.ceiling_lamp_off")
      (Development|PrintString "is on"))))