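; Level 3 decal dot that slides along the paper actor it is attached to, at a set speed.
; SetMultipleFloats sets speed, start, size and dynamic-material opacity, and caches the parent paper's bounds and scale; SetBool starts or stops movement.
; Tick advances a clamped relative X, which Rel2Abs converts into a decal offset using those bounds.
; Radial diffusion and linear stretch helpers exist but their EventGraph calls never run.
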(event EventSetBool
  (params (Bool :type Boolean))
  (Variables|Default|SetIs%20Running Bool))

(event EventTick
  (params (DeltaSeconds :type Float%20%28single-precision%29))
  (if (Variables|Default|GetIs%20Running)
    ;[1 1 1] Set new relative location
    (Variables|Default|SetDot%20Loc%20Rel (Math|Vector|MakeVector (Math|Float|Clamp(Float) (+ (* DeltaSeconds (Variables|Default|GetSpeed%20Dot)) (.x (Variables|Default|GetDot%20Loc%20Rel))) 0.2 1.8) (.y (Variables|Default|GetDot%20Loc%20Rel)) (.z (Variables|Default|GetDot%20Loc%20Rel))))
    (Transformation|SetRelativeLocation (Variables|Decal|GetDecal) (Math|Vector|MakeVector (CallFunction|Rel2Abs (+ (* DeltaSeconds (Variables|Default|GetSpeed%20Dot)) (.x (Variables|Default|GetDot%20Loc%20Rel))) (.x (Variables|Default|GetPaper%20Bounds)) (.x (Variables|Default|GetPaper%20Scale))) 0.0 0.0) false false)))

(event EventSetMultipleFloats
  (params (Float :type Array%20of%20Floats%20%28double-precision%29))
  (bind _returnvalue (Class|Actor|GetActorRelativeScale3D))
  (bind _rootcomponent (Variables|Transformation|GetRootComponent))
  (bind _returnvalue_2 (Transformation|GetAttachParent _rootcomponent))
  (bind _returnvalue_3 (Components|GetOwner _returnvalue_2))
  (Variables|Default|SetSpeed%20Dot (Utilities|Array|Get(acopy) Float))
  (Variables|Default|SetDot%20Loc%20Rel (Math|Vector|MakeVector (Utilities|Array|Get(acopy) Float 1) 0.5 0.5))
  (Variables|Default|SetDot%20Radius (Utilities|Array|Get(acopy) Float 2))
  (Variables|Default|SetOpacity (Utilities|Array|Get(acopy) Float 3))
  (bind _output_get (Variables|Default|SetPaper%20Bounds (.BoxExtent (Collision|GetActorBounds _returnvalue_3 false false))))
  (bind _output_get_2 (Variables|Default|SetPaper%20Scale (Transformation|GetActorScale3D _returnvalue_3)))
  (Development|PrintString (Utilities|String|ToString(Vector) _output_get_2))
  (Development|PrintString (Utilities|String|ToString(Vector) _output_get))
  (Transformation|SetActorRelativeScale3D (Math|Vector|MakeVector (.x _returnvalue) (Math|Float|Clamp(Float) (* (.y _returnvalue) (Variables|Default|GetDot%20Radius)) 0.0 1e+01) (Math|Float|Clamp(Float) (* (.z _returnvalue) (Variables|Default|GetDot%20Radius)) 0.0 1e+01)))
  (Rendering|Material|SetScalarParameterValue (Variables|Default|Getcolor) "opacity" (Variables|Default|GetOpacity) :!class /Script/Engine.MaterialInstanceDynamic))

(fn ConstructionScript
  (bind _returnvalue (Rendering|Material|CreateDynamicMaterialInstance (Variables|Decal|GetDecal) :!class /Script/Engine.DecalComponent))
  (Variables|Default|Setcolor _returnvalue))

(fn RadialDiffusionDot
  (params (Delta%20Time :type Float%20%28double-precision%29%20%28by%20ref%29) (Start%20Radius%20Rel :type Float%20%28double-precision%29) (Max%20Radius%20Rel :type Float%20%28double-precision%29) (Radial%20Diffusion%20Speed :type Float%20%28double-precision%29))
  (bind _output_get (Variables|Default|SetDot%20Radius (Math|Float|Clamp(Float) (+ (* Radial%20Diffusion%20Speed Delta%20Time) (Variables|Default|GetDot%20Radius)) Start%20Radius%20Rel Max%20Radius%20Rel)))
  (Transformation|SetRelativeScale3D (Variables|Decal|GetDecal) (Math|Vector|MakeVector 0.1 _output_get _output_get)))

(fn CalcLocationAbs
  (params (Delta%20Time :type Float%20%28double-precision%29%20%28by%20ref%29) (Speed%20Dot%20Rel :type Float%20%28double-precision%29))
  (bind _paper_bounds (Variables|Default|GetPaper%20Bounds))
  (bind _paper_scale (Variables|Default|GetPaper%20Scale))
  (bind _dot_loc_rel (Variables|Default|GetDot%20Loc%20Rel))
  (bind _paper_bounds_2 (Variables|Default|GetPaper%20Bounds))
  (bind _returnvalue (/ (.x _paper_bounds) (.x _paper_scale)))
  (bind _returnvalue_2 (* _returnvalue 1.8))
  (return (Math|Vector|MakeVector (* (Math|Float|Clamp(Float) (+ (* Delta%20Time Speed%20Dot%20Rel) (.x _dot_loc_rel)) _returnvalue_2 (* _returnvalue_2 -1.0)) (.x _paper_bounds_2)) (* (.y _paper_bounds_2) (.y _dot_loc_rel)) (* (.z _paper_bounds_2) (.z _dot_loc_rel)))))

(fn CalcLinearStretch
  (params (Delta%20Time :type Float%20%28double-precision%29%20%28by%20ref%29) (Dot%20Strech%20Speed :type Float%20%28double-precision%29) (Dot%20Max%20Stretch :type Float%20%28double-precision%29))
  (bind _paper_scale (Variables|Default|GetPaper%20Scale))
  (bind _output_get (Variables|Default|SetDot%20Strech (Math|Float|Clamp(Float) (+ (* Delta%20Time Dot%20Strech%20Speed) (.z _paper_scale)) 1.0 Dot%20Max%20Stretch)))
  (Transformation|SetRelativeScale3D (Variables|Decal|GetDecal) (Math|Vector|MakeVector (.x _paper_scale) (.y _paper_scale) _output_get)))

(fn CalcAbsLocationfromPerc
  (params (Rel%20X :type Float%20%28double-precision%29) (Rel%20Y :type Float%20%28double-precision%29) (Rel%20Z :type Float%20%28double-precision%29))
  (bind _returnvalue (* Rel%20X 2.0))
  (bind _returnvalue_2 (* Rel%20Z 2.0))
  (bind _returnvalue_3 (* Rel%20Y 2.0))
  (bind _paper_bounds (Variables|Default|GetPaper%20Bounds))
  (bind _paper_scale (Variables|Default|GetPaper%20Scale))
  (bind _returnvalue_4 (- _returnvalue 1.0))
  (bind _returnvalue_5 (- _returnvalue_2 1.0))
  (bind _returnvalue_6 (- _returnvalue_3 1.0))
  (bind _returnvalue_7 (* (.x _paper_bounds) _returnvalue_4))
  (bind _returnvalue_8 (* (.z _paper_bounds) _returnvalue_5))
  (bind _returnvalue_9 (* (.y _paper_bounds) _returnvalue_6))
  (return (Math|Float|Lerp (/ _returnvalue_7 (.x _paper_scale)) (/ _returnvalue_7 (.x _paper_scale)) Rel%20X) (Math|Float|Lerp (/ _returnvalue_9 (.y _paper_scale)) (/ _returnvalue_9 (.y _paper_scale)) Rel%20Y) (Math|Float|Lerp (/ _returnvalue_8 (.z _paper_scale)) (/ _returnvalue_8 (.z _paper_scale)) Rel%20Z)))

(fn Rel2Abs
  (params (Rel :type Float%20%28double-precision%29) (Tot :type Float%20%28double-precision%29) (Scale :type Float%20%28double-precision%29))
  (return (* (- Rel 1.0) (/ Tot Scale))))