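; BP_Paperholder is a paper holder that receives an item carried by the player's held tweezers (BP_Pinzette).
; Its Combine event checks that the player holds tweezers with exactly one directly attached actor.
; It then reattaches that actor to itself at socket "1", snapping location, rotation and scale to the target.
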(event EventCombine
  (params (HitComp :type Primitive%20Component%20Object%20Reference) (PhysicsHandle :type Physics%20Handle%20Component%20Object%20Reference))
  (bind _held_actor (CallFunction|GetHeldActor))
  (bind _outactors (Actor|GetAttachedActors _held_actor true false))
  (if (CallFunction|PlayerIsHolding)
    (if (== (CallFunction|GetHeldActorType) "/Game/0_MY_STUFF/BP_Pinzette.BP_Pinzette_C")
      (if (== (Utilities|Array|Length _outactors) 1)
        (Transformation|AttachActorToActor (Utilities|Array|Get(acopy) _outactors) self "1" "SnapToTarget" "SnapToTarget" "SnapToTarget" true)))))

(fn ConstructionScript)