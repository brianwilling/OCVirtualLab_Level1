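; BP_Sink is a sink Blueprint with left and right doors that toggle between two positions.
; Its Combine event receives a hit component and matches it against RightDoor or LeftDoor.
; Each door has its own FlipFlop that instantly rotates it 90 degrees one way, then back on the next call, mirrored between sides.
; Debug prints report which side was hit.
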(event EventCombine
  (params (HitComp :type Primitive%20Component%20Object%20Reference) (PhysicsHandle :type Physics%20Handle%20Component%20Object%20Reference))
  (if (== (Variables|Default|GetRight%20Door) HitComp)
    (Development|PrintString "right")
    (Utilities|FlowControl|FlipFlop
      (:A
        (Transformation|AddLocalRotation HitComp "0,-90.000000, 0" false false))
      (:B
        (Transformation|AddLocalRotation HitComp "0,90.000000, 0" false false)))
    (elif (== (Variables|Default|GetLeft%20Door) HitComp)
      (Development|PrintString "left")
      (Utilities|FlowControl|FlipFlop
        (:A
          (Transformation|AddLocalRotation HitComp "0,90.000000, 0" false false))
        (:B
          (Transformation|AddLocalRotation HitComp "0,-90.000000, 0" false false))))))

(fn ConstructionScript)