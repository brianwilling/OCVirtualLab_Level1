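; BP_DC_UV_Lamp is an interactable UV lamp that toggles its light and can hold a paper.
; Combine checks for held level 2 tweezers (BP_Pinzette_LVL2), moving their single attached actor onto the lamp, or returning the lamp's paper otherwise, via "Paper" sockets and HasPaper.
; Other interactions call LightSwitch, which flips IsOn and RectLight intensity with debug prints.
; The construction script applies ON intensity when IsOn is set.
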(event Custom|LightSwitch
  (if (Variables|Default|GetIsOn)
    (Rendering|Components|Light|SetIntensity (Variables|Default|GetRectLight) 0.0)
    (Development|PrintString "OFF")
    (Variables|Default|SetIsOn false)
    (else
      (Rendering|Components|Light|SetIntensity (Variables|Default|GetRectLight) (Variables|Default|GetON%20Intensity))
      (Development|PrintString "ON")
      (Variables|Default|SetIsOn true))))

(event EventCombine
  (params (HitComp :type Primitive%20Component%20Object%20Reference) (PhysicsHandle :type Physics%20Handle%20Component%20Object%20Reference))
  (bind _held_actor (CallFunction|GetHeldActor))
  (bind _outactors (Actor|GetAttachedActors _held_actor true false))
  (if (CallFunction|PlayerIsHolding)
    (if (== (CallFunction|GetHeldActorType) "/Game/0_MY_STUFF/BP_Pinzette_LVL2.BP_Pinzette_LVL2_C")
      (if (== (Utilities|Array|Length _outactors) 1)
        (Transformation|AttachActorToActor (Utilities|Array|Get(acopy) _outactors) self "Paper" "SnapToTarget" "SnapToTarget" "SnapToTarget" true)
        (Variables|Default|SetHas%20Paper true)
        (elif (Variables|Default|GetHas%20Paper)
          (Transformation|AttachActorToActor (Utilities|Array|Get(acopy) (Actor|GetAttachedActors true false)) (CallFunction|GetHeldActor) "Paper" "SnapToTarget" "SnapToTarget" "SnapToTarget" true)
          (Variables|Default|SetHas%20Paper false)
          (else
            (CallFunction|LightSwitch))))
      (else
        (CallFunction|LightSwitch)))
    (else
      (CallFunction|LightSwitch))))

(fn ConstructionScript
  (if (Variables|Default|GetIsOn)
    (Rendering|Components|Light|SetIntensity (Variables|Default|GetRectLight) (Variables|Default|GetON%20Intensity))
    (Development|PrintString "is on")))