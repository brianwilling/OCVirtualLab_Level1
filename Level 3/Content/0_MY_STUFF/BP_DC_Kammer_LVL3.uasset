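; BP_DC_Kammer_LVL3 is a lab chamber, likely for thin-layer chromatography, that takes paper and liquid and has a toggleable lid.
; When open, Combine moves paper to or from held tweezers via socket attachment, or shows fluid for a held beaker; otherwise it toggles the lid.
; Lid changes and paper insertion send bool messages to the paper or its attachments.
; The construction script sets fluid visibility and positions the lid inversely to IsOpen.
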(event Custom|open/close%20lid
  (bind _paper (Variables|Default|GetPaper))
  (bind _outactors (Actor|GetAttachedActors _paper true false))
  (if (Variables|Default|GetIs%20Open)
    ;[1 1 1] close lid
    (Transformation|SetRelativeLocation (Variables|Default|GetLid) (Variables|Default|GetClosedLidLocation) false false)
    (Variables|Default|SetIs%20Open false)
    (Development|PrintString "Closing chamber")
    (if (and (Variables|Default|GetHasLiquid) (Variables|Default|GetHasPaper))
      (for _array_element _outactors
        (Class|BPISetBool|SetBool(Message) _array_element true)
        (Development|PrintString "is setting bool")
        (Class|BPISetBool|SetBool(Message) (Variables|Default|GetPaper) true)))
    (else
      ;[1 1 1] open lid
      (Transformation|SetRelativeLocation (Variables|Default|GetLid) (Variables|Default|GetOpenedLidLocation) false false)
      (Variables|Default|SetIs%20Open true)
      (Development|PrintString "Opening chamber")
      (if (Variables|Default|GetHasPaper)
        (for _array_element_2 _outactors
          (Class|BPISetBool|SetBool(Message) _array_element_2 false)
          (Class|BPISetBool|SetBool(Message) (Variables|Default|GetPaper) false))))))

(event EventCombine
  (params (HitComp :type Primitive%20Component%20Object%20Reference) (PhysicsHandle :type Physics%20Handle%20Component%20Object%20Reference))
  ;[1 1 1] Is Holding and Open?
  (if (and (CallFunction|PlayerIsHolding) (Variables|Default|GetIs%20Open))
    ;[1 1 1] Holding Pinzette
    (if (== (CallFunction|GetHeldActorType) "/Game/0_MY_STUFF/BP_Pinzette.BP_Pinzette_C")
      ;[1 1 1] has Paper?
      (if (Variables|Default|GetHasPaper)
        ;[1 1 1] Paper to Pinzette
        (Transformation|AttachActorToActor (Variables|Default|GetPaper) (CallFunction|GetHeldActor) "Paper" "SnapToTarget" "SnapToTarget" "SnapToTarget" true)
        (Variables|Default|SetHasPaper false)
        (Variables|Default|SetPaper 0)
        (else
          ;[1 1 1] Paper to Chamber
          (bind _output_get (Variables|Default|SetPaper (Utilities|Array|Get(acopy) (Actor|GetAttachedActors (CallFunction|GetHeldActor) true false))))
          (Transformation|AttachActorToActor _output_get self "Paper" "SnapToTarget" "SnapToTarget" "SnapToTarget" true)
          (Variables|Default|SetHasPaper true)
          (if (Variables|Default|GetHasLiquid)
            (Class|BPISetBool|SetBool(Message) (Variables|Default|GetPaper) true))))
      (else
        ;[1 1 1] Holding Becherglas
        (if (== (CallFunction|GetHeldActorType) "/Game/0_MY_STUFF/BP_Becherglas.BP_Becherglas_C")
          (Development|PrintString "fill with liquid")
          (Rendering|SetVisibility (Variables|Default|GetFluid) true false)
          (Variables|Default|SetHasLiquid true)
          (else
            (CallFunction|Open/closeLid)
            (Development|PrintString "not holding relevant actor")))))
    (else
      (CallFunction|Open/closeLid))))

(fn ConstructionScript
  (Rendering|SetVisibility (Variables|Default|GetFluid) (Variables|Default|GetHasLiquid) false)
  (if (Variables|Default|GetIs%20Open)
    (Transformation|SetRelativeLocation (Variables|Default|GetLid) (Variables|Default|GetClosedLidLocation) false false)
    (else
      (Transformation|SetRelativeLocation (Variables|Default|GetLid) (Variables|Default|GetOpenedLidLocation) false false))))