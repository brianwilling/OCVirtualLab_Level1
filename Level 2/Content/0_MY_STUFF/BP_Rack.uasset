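; BP_Rack is an interactive prop with a faucet valve that switches a steam effect on and off.
; Each Combine event alternates through a FlipFlop, rotating the valve 15 degrees one way or back.
; Switching on spawns an auto-release pooled P_Steam_Lit emitter at the SteamEmitter location and prints a debug message.
; Switching off deactivates that spawned emitter.
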(event EventCombine
  (params (HitComp :type Primitive%20Component%20Object%20Reference) (PhysicsHandle :type Physics%20Handle%20Component%20Object%20Reference))
  (Utilities|FlowControl|FlipFlop
    (:A
      (Transformation|AddLocalRotation (Variables|Default|GetFaucet%20Valve) "0,0.000000,-15.000000" false false)
      (bind _returnvalue (Effects|SpawnEmitteratLocation "/Game/StarterContent/Particles/P_Steam_Lit.P_Steam_Lit" (Transformation|GetWorldLocation (Variables|Default|GetSteam%20Emitter)) "0, 0, 0" (Variables|Default|GetScale) true "AutoRelease"))
      (Development|PrintString "ON" true true "(R=0.075834,G=1.000000,B=0.000000,A=1.000000)"))
    (:B
      (Transformation|AddLocalRotation (Variables|Default|GetFaucet%20Valve) "0,0.000000,15.000000" false false)
      (Components|Activation|Deactivate _returnvalue))))

(fn ConstructionScript)