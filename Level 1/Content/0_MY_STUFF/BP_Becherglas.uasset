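; BP_Becherglas is an interactable beaker actor that shows or hides its Widget when interacted with.
; The interface interact call forwards to InteractOnServer, which flips InteractToggle.
; The OnRep for that boolean sets the Widget's visibility, keeping the toggle replicated across the network.
; Focus changes only print a debug string, and the interaction widget getter returns nothing.
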(event Custom|InteractOnServer
  (Variables|Default|SetInteractToggle (not (Variables|Default|GetInteractToggle))))

(event EventInterfaceToggleFocus
  (params (Fokus :type Boolean))
  (Development|PrintString (Utilities|String|ToString(Boolean) Fokus) true true "(R=1.000000,G=0.345643,B=0.584464,A=1.000000)"))

(event EventInterfaceInteract
  (CallFunction|InteractonServer))

(fn ConstructionScript)

(fn OnRepInteractToggle
  (bind _widget (Variables|Default|GetWidget))
  (if (Variables|Default|GetInteractToggle)
    (Rendering|SetVisibility _widget true false)
    (else
      (Rendering|SetVisibility _widget false false))))

(fn GetInteractionWidgetref
  (return 0))