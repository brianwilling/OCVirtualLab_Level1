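; Placement slot actor that accepts a held item of a specific class, marked by a decal.
; Combine checks the player's held actor against TypeSlot and, if the slot is free, positions and rotates it, attaches it, hides the decal and releases the player's physics handle.
; SetBool toggles the decal's visibility.
; The construction script sizes the VisibilityBlocker box to match the decal.
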(event EventSetBool
  (params (Bool :type Boolean))
  (Development|PrintString "settiong")
  (Rendering|SetVisibility (Variables|Decal|GetDecal) Bool false))

(event EventCombine
  (params (HitComp :type Primitive%20Component%20Object%20Reference) (PhysicsHandle :type Physics%20Handle%20Component%20Object%20Reference))
  (Development|PrintString "dododod")
  ;[1 1 1] Player is holding an item
  (if (CallFunction|PlayerIsHolding)
    (Development|PrintString "checking type")
    (Variables|Default|SetTypeHeld (Utilities|GetClass (CallFunction|GetHeldActor)))
    (if (and (not (Variables|Default|GetIsOccupied)) (== (Variables|Default|GetTypeSlot) (Variables|Default|GetTypeHeld)))
      (Development|PrintString "trying to attach")
      (bind _output_get (Variables|Default|SetActorInSlot (CallFunction|GetHeldActor)))
      (Transformation|SetActorLocationAndRotation _output_get (Transformation|GetWorldLocation (Variables|Decal|GetDecal)) (Variables|Default|GetSlotRotation))
      (Transformation|AttachActorToActor _output_get self "None" "SnapToTarget" "KeepWorld" "KeepWorld" false)
      (Variables|Default|SetIsOccupied true)
      (Rendering|SetVisibility (Variables|Decal|GetDecal) false false)
      (Physics|Components|PhysicsHandle|ReleaseComponent (Actor|GetComponentbyClass (Game|Player|GetPlayerPawn 0) "/Script/Engine.PhysicsHandleComponent")))
    (elif true
      _)))

(fn ConstructionScript
  (bind _decal (Variables|Decal|GetDecal))
  (bind _decalsize (Variables|/Script/Engine.DecalComponent|GetDecalSize _decal))
  (Components|Box|SetBoxExtent (Variables|Default|GetVisibility%20Blocker) (Math|Vector|MakeVector (.x _decalsize) (.y _decalsize) (.z _decalsize)) true))