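; BP_PaperStand is a stand that receives a paper from, or returns it to, the tweezers (BP_Pinzette) held by the player.
; The Combine event uses two helper checks for whether the held item is a pinzette and whether it carries a BP_Paper.
; It then snaps the paper between the pinzette and the stand's "Paper" socket, tracking it with StandHasPaper and an AttachedPaper reference.
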(event EventCombine
  (params (HitComp :type Primitive%20Component%20Object%20Reference) (PhysicsHandle :type Physics%20Handle%20Component%20Object%20Reference))
  (Variables|Default|SetPinzette%20Has%20Paper (CallFunction|GetPinzetteHasPaper))
  (Variables|Default|SetIs%20Holding%20Pinzette (CallFunction|GetIsHoldingPinzette))
  ;[1 1 1] Attach Paper if true
  (if (and (Variables|Default|GetPinzette%20Has%20Paper) (not (Variables|Default|GetStand%20Has%20Paper)))
    (bind _output_get (Variables|Default|SetAttached%20Paper (Utilities|Array|Get(acopy) (Actor|GetAttachedActors (CallFunction|GetHeldActor) true false))))
    (Transformation|AttachActorToActor _output_get self "Paper" "SnapToTarget" "SnapToTarget" "SnapToTarget" true)
    (Variables|Default|SetStand%20Has%20Paper true)
    (else
      ;[1 1 1] Detach Paper if True
      (if (and (Variables|Default|GetIs%20Holding%20Pinzette) (Variables|Default|GetStand%20Has%20Paper))
        (Transformation|AttachActorToActor (Utilities|Array|Get(acopy) (Actor|GetAttachedActors true false)) (CallFunction|GetHeldActor) "Paper" "SnapToTarget" "SnapToTarget" "SnapToTarget" true)
        (Variables|Default|SetStand%20Has%20Paper false)
        ;[1 1 1] Clear Actor reference
        (Variables|Default|SetAttached%20Paper 0)))))

(fn ConstructionScript)

(fn GetPinzetteHasPaper
  (if (CallFunction|PlayerIsHolding)
    (if (== (Utilities|GetClass (CallFunction|GetHeldActor)) "/Game/0_MY_STUFF/BP_Pinzette.BP_Pinzette_C")
      (if (== (Utilities|Array|Length (Actor|GetAttachedActors (CallFunction|GetHeldActor) true false)) 1)
        (if (or (== (Utilities|GetClass (Utilities|Array|Get(acopy) (Actor|GetAttachedActors (CallFunction|GetHeldActor) true false))) "/Game/0_MY_STUFF/BP_Paper.BP_Paper_C") false)
          (return true)
          (else
            (return false)))
        (else
          (return false)))
      (else
        (return false)))
    (else
      (return false))))

(fn GetIsHoldingPinzette
  (if (CallFunction|PlayerIsHolding)
    (if (== (Utilities|GetClass (CallFunction|GetHeldActor)) "/Game/0_MY_STUFF/BP_Pinzette.BP_Pinzette_C")
      (return true)
      (else
        (return false)))
    (else
      (return false))))