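; Chromatography paper actor that responds to the held tool via Combine.
; Tweezers pick it up, a filled capillary spawns two attached BP_DC_Dot actors with solvent-specific speeds, and a pencil reveals the baseline, plus a solvent-front line once wetting has run.
; SetBool starts or stops the dots, while a timeline advances the wetting liquid.
; Dot placement converts relative percentages to local coordinates from actor bounds.
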(event Custom|Event%20movingLiquidPlaced
  ;[1 1 1] wetting of the paper when standing in beaker
  (Rendering|SetVisibility (Variables|Default|GetmovingLiquid) true false))

(event Custom|Event%20movingLiquidRunning
  (bind _default_location_movingliquid (Variables|Default|GetDefault%20Location%20MovingLiquid))
  ;[1 1 1] wetting of paper when DC-chamber closed
  (if (Variables|Default|GetMovingLiquidRunning)
    (bind _runliquid (Timeline|TL%20movingLiquid Play)
      (:Update
        (Transformation|SetRelativeLocation (Variables|Default|GetmovingLiquid) (Math|Vector|MakeVector (Math|Float|Lerp (.x _default_location_movingliquid) 0.0 _runliquid) (.y _default_location_movingliquid) (.z _default_location_movingliquid)) false false)
        (Variables|Default|SetMovingLiquidRunningStarted true)))
    (else
      (Timeline|TL%20movingLiquid Stop))))

(event EventSetBool
  (params (Bool :type Boolean))
  (for _array_element (Actor|GetAttachedActors true false)
    (bind _asbp_dc_dot (Utilities|Casting|CastToBP_DC_Dot _array_element))
    (Variables|/Game/0_MY_STUFF/BP_DC_Dot.BP_DC_Dot_C|SetIs%20Running _asbp_dc_dot Bool)))

(event EventCombine
  (params (HitComp :type Primitive%20Component%20Object%20Reference) (PhysicsHandle :type Physics%20Handle%20Component%20Object%20Reference))
  (bind _movingliquid (Variables|Default|GetmovingLiquid))
  (bind _returnvalue (Transformation|GetRelativeTransform _movingliquid))
  (if (CallFunction|PlayerIsHolding)
    (if (== (CallFunction|GetHeldActorType) "/Game/0_MY_STUFF/BP_Pinzette.BP_Pinzette_C")
      (if (== (Utilities|Array|Length (Actor|GetAttachedActors (CallFunction|GetHeldActor) true false)) 0)
        (Transformation|AttachActorToActor self (CallFunction|GetHeldActor) "Paper" "SnapToTarget" "SnapToTarget" "SnapToTarget" true)
        (else
          (Development|PrintString "pinzette has a paper")))
      (elif (== (CallFunction|GetHeldActorType) "/Game/0_MY_STUFF/BP_Capillary.BP_Capillary_C")
        (bind _asbp_capillary (Utilities|Casting|CastToBP_Capillary (CallFunction|GetHeldActor))
          (:then
            (if (Variables|/Game/0_MY_STUFF/BP_Capillary.BP_Capillary_C|GetIs%20Filled _asbp_capillary)
              (if (== (Utilities|Array|Length (Actor|GetAttachedActors true false)) 0)
                (if (== (Variables|Default|GetZählvarDecal) 0)
                  (bind (_decal _spawn_actor_location) (Utilities|AttachDecal))
                  ;[1 1 1] Set the start location and speed of DC dot
                  (Class|BPISetVec|SetVec(Message) _decal _spawn_actor_location)
                  (Class|BPISetMultipleFloats|SetMultipleFloats(Message) _decal (Utilities|Array|MakeArray (.speeda_out (CallFunction|GetSolventProps (Variables|/Game/0_MY_STUFF/BP_Capillary.BP_Capillary_C|GetSolution%20Type _asbp_capillary))) 0.1))
                  (bind (_decal_2 _spawn_actor_location_2) (Utilities|AttachDecal))
                  (Class|BPISetVec|SetVec(Message) _decal_2 _spawn_actor_location_2)
                  (Class|BPISetMultipleFloats|SetMultipleFloats(Message) _decal_2 (Utilities|Array|MakeArray (.speedb_out (CallFunction|GetSolventProps (Variables|/Game/0_MY_STUFF/BP_Capillary.BP_Capillary_C|GetSolution%20Type _asbp_capillary))) 0.1))
                  (Variables|Default|SetZählvarDecal 1)
                  (if (== (Variables|Default|GetZählvarDecal) 1)
                    (Rendering|SetVisibility (Variables|Default|GetDecal1) true false)
                    (Variables|Default|SetZählvarDecal 0)))
                (else
                  (Development|PrintString "open clos")))
              (else
                (Development|PrintString "capillary empty"))))
          (:CastFailed
            (Development|PrintString "cast failed to capillary")))
        (elif (== (CallFunction|GetHeldActorType) "/Game/0_MY_STUFF/BP_Pencil.BP_Pencil_C")
          (Rendering|SetVisibility (Variables|Default|Getline%20bottom) true false)
          (if (Variables|Default|GetMovingLiquidRunningStarted)
            (Transformation|SetRelativeLocation (Variables|Default|Getline%20top) (Math|Vector|MakeVector (+ (.x (.location _returnvalue)) 4.7) (.y (.location _returnvalue)) (.z (.location _returnvalue))) false false)
            (Rendering|SetVisibility (Variables|Default|Getline%20top) true false))
          (else
            (Development|PrintString "Do Nothing")))))
    (else
      (Development|PrintString "do nothing"))))

(fn ConstructionScript
  (bind _decal (Variables|Default|GetDecal))
  (bind _start_radius_rel (Variables|Default|GetStart%20Radius%20Rel))
  (bind _start_loc_perc (Variables|Default|GetStart%20Loc%20Perc))
  (bind (_abs_x _abs_y _abs_z) (CallFunction|CalcAbsLocationfromPerc _start_loc_perc 0.3 0.5))
  (Transformation|SetRelativeLocationAndRotation _decal (Math|Vector|MakeVector _abs_x _abs_y _abs_z) "90.000000,180.000000, 0" false false)
  (Transformation|SetRelativeScale3D _decal (Math|Vector|MakeVector 0.001 _start_radius_rel _start_radius_rel))
  (Variables|Default|SetDefault%20Location%20MovingLiquid (.location (Transformation|GetRelativeTransform (Variables|Default|GetmovingLiquid)))))

(fn PropagateDot
  (params (Delta%20Time :type Float%20%28double-precision%29%20%28by%20ref%29) (Dot%20Decal :type Decal%20Component%20Object%20Reference%20%28by%20ref%29) (Start%20Position%20Rel :type Float%20%28double-precision%29) (End%20Position%20Rel :type Float%20%28double-precision%29) (Speed%20Abs :type Float%20%28double-precision%29))
  (bind _output_get (Variables|Default|SetDotLocation (Math|Float|Clamp(Float) (+ (* Speed%20Abs Delta%20Time) (Variables|Default|GetDotLocation)) (.Abs%20X (CallFunction|CalcAbsLocationfromPerc Start%20Position%20Rel 0.0 0.0)) (.Abs%20X (CallFunction|CalcAbsLocationfromPerc End%20Position%20Rel 0.0 0.0)))))
  (Transformation|SetRelativeLocation Dot%20Decal (Math|Vector|MakeVector _output_get 0.0 0.0) false false))

(fn CalcAbsLocationfromPerc
  (params (Rel%20X :type Float%20%28double-precision%29) (Rel%20Y :type Float%20%28double-precision%29) (Rel%20Z :type Float%20%28double-precision%29))
  (bind _boxextent (Collision|GetActorBounds false false))
  (bind _returnvalue (Class|Actor|GetActorRelativeScale3D))
  (bind _returnvalue_2 (* Rel%20X 2.0))
  (bind _returnvalue_3 (* Rel%20Z 2.0))
  (bind _returnvalue_4 (* Rel%20Y 2.0))
  (bind _returnvalue_5 (- _returnvalue_2 1.0))
  (bind _returnvalue_6 (- _returnvalue_3 1.0))
  (bind _returnvalue_7 (- _returnvalue_4 1.0))
  (bind _returnvalue_8 (* (.x _boxextent) _returnvalue_5))
  (bind _returnvalue_9 (* (.z _boxextent) _returnvalue_6))
  (bind _returnvalue_10 (* (.y _boxextent) _returnvalue_7))
  (return (Math|Float|Lerp (/ _returnvalue_8 (.x _returnvalue)) (/ _returnvalue_8 (.x _returnvalue)) Rel%20X) (Math|Float|Lerp (/ _returnvalue_10 (.y _returnvalue)) (/ _returnvalue_10 (.y _returnvalue)) Rel%20Y) (Math|Float|Lerp (/ _returnvalue_9 (.z _returnvalue)) (/ _returnvalue_9 (.z _returnvalue)) Rel%20Z)))

(fn RadialDiffusionDot
  (params (Delta%20Time :type Float%20%28double-precision%29%20%28by%20ref%29) (Dot%20Decal :type Decal%20Component%20Object%20Reference%20%28by%20ref%29) (Start%20Radius%20Rel :type Float%20%28double-precision%29) (Max%20Radius%20Rel :type Float%20%28double-precision%29) (Radial%20Diffusion%20Speed :type Float%20%28double-precision%29))
  (bind _output_get (Variables|Default|SetDot%20Radius (Math|Float|Clamp(Float) (+ (* Radial%20Diffusion%20Speed Delta%20Time) (Variables|Default|GetDot%20Radius)) Start%20Radius%20Rel Max%20Radius%20Rel)))
  (Transformation|SetRelativeScale3D Dot%20Decal (Math|Vector|MakeVector 0.1 _output_get _output_get)))

(fn CalcLinearStretch
  (params (Delta%20Time :type Float%20%28double-precision%29%20%28by%20ref%29) (Dot%20Decal :type Decal%20Component%20Object%20Reference%20%28by%20ref%29) (Dot%20Strech%20Speed :type Float%20%28double-precision%29) (Dot%20Max%20Stretch :type Float%20%28double-precision%29))
  (bind _relativescale3d (Variables|/Script/Engine.SceneComponent|GetRelativeScale3D Dot%20Decal))
  (bind _output_get (Variables|Default|SetDot%20Strech%20Scale (Math|Float|Clamp(Float) (+ (* Delta%20Time Dot%20Strech%20Speed) (.z _relativescale3d)) 1.0 Dot%20Max%20Stretch)))
  (Transformation|SetRelativeScale3D Dot%20Decal (Math|Vector|MakeVector (.x _relativescale3d) (.y _relativescale3d) _output_get)))

(fn NewFunction)