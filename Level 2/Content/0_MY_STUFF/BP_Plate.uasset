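; BP_Plate is a plate that exchanges a paper with BP_Pinzette_LVL2 tweezers held by player 0.
; Its Combine event checks the held tweezers' attachment count: at exactly one, it reads index 1 and snaps that entry to the plate's Paper socket.
; Otherwise, if HasPaper is set, the plate's first attached actor snaps to the tweezers' Paper socket.
; HasPaper flips with each transfer.
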(event EventCombine
  (params (HitComp :type Primitive%20Component%20Object%20Reference) (PhysicsHandle :type Physics%20Handle%20Component%20Object%20Reference))
  (bind _held_actor (CallFunction|GetHeldActor))
  (bind _outactors (Actor|GetAttachedActors _held_actor true false))
  (if (CallFunction|PlayerIsHolding)
    (if (== (CallFunction|GetHeldActorType) "/Game/0_MY_STUFF/BP_Pinzette_LVL2.BP_Pinzette_LVL2_C")
      (if (== (Utilities|Array|Length _outactors) 1)
        (Transformation|AttachActorToActor (Utilities|Array|Get(acopy) _outactors 1) self "Paper" "SnapToTarget" "SnapToTarget" "SnapToTarget" true)
        (Variables|Default|SetHasPaper true)
        (elif (Variables|Default|GetHasPaper)
          (Transformation|AttachActorToActor (Utilities|Array|Get(acopy) (Actor|GetAttachedActors true false)) (CallFunction|GetHeldActor) "Paper" "SnapToTarget" "SnapToTarget" "SnapToTarget" true)
          (Variables|Default|SetHasPaper false))))))

(fn ConstructionScript)